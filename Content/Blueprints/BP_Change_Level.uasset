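; BP_Change_Level alternates turns between two players by timing each level run and loading the Switch_Players level.
; On BeginPlay it flips the Player2 flag in B_CBBAInstance, raising Difficulty (capped at 3) whenever the flag returns to false.
; Tick accumulates SwitchTimer only while the player character is alive, then opens Switch_Players by name once it passes thirty seconds.
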(event `self.ReceiveBeginPlay`
  (bind _asb_cbbainstance (cast `/Game/Player/Blueprints/B_CBBAInstance` (`GameplayStatics.GetGameInstance`)))
  (if (`/Game/Player/Blueprints/B_CBBAInstance.Player2` _asb_cbbainstance)
    (set `/Game/Player/Blueprints/B_CBBAInstance.Player2` false _asb_cbbainstance)
    (bind _difficulty (`/Game/Player/Blueprints/B_CBBAInstance.Difficulty` _asb_cbbainstance))
    (if (< _difficulty 3)
      (set `/Game/Player/Blueprints/B_CBBAInstance.Difficulty` (+ _difficulty 1) _asb_cbbainstance))
    (else
      (set `/Game/Player/Blueprints/B_CBBAInstance.Player2` true _asb_cbbainstance))))

(event `self.ReceiveTick`
  (params (DeltaSeconds :type "Float (single-precision)"))
  (bind _asb_cbbaplayer_character (cast `/Game/Player/Blueprints/B_CBBAPlayerCharacter` (`GameplayStatics.GetPlayerPawn` 0)))
  (if (not (`/Game/Player/Blueprints/B_CBBAPlayerCharacter.IsDead` _asb_cbbaplayer_character))
    (bind _output_get (set `self.SwitchTimer` (+ DeltaSeconds (`self.SwitchTimer`))))
    (if (> _output_get 30.0)
      (`GameplayStatics.OpenLevel` "Switch_Players"))))

(fn `UserConstructionScript`)