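; Spawner actor that repeatedly creates bleachers at its own location.
; The Rotate flag selects BP_Bleachers_Rotated with a fixed 180-degree rotation, or BP_Bleachers with default rotation.
; BeginPlay spawns the first one immediately.
; Tick drives further spawns through a Delay of SpawnDelay plus frame time, which ignores calls while pending and so acts as a repeating timer.
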(event `self.ReceiveBeginPlay`
  (bind _returnvalue (`self.K2_GetActorLocation`))
  (if (`self.Rotate`)
    (`|SpawnActorFromClass` "/Game/Blueprints/BP_Bleachers_Rotated.BP_Bleachers_Rotated_C" (`KismetMathLibrary.MakeTransform` _returnvalue (struct :`Yaw` 180.0)) "Undefined" "MultiplyWithRoot" null null)
    (else
      (`|SpawnActorFromClass` "/Game/Blueprints/BP_Bleachers.BP_Bleachers_C" (`KismetMathLibrary.MakeTransform` _returnvalue) "Undefined" "MultiplyWithRoot" null null))))

(event `self.ReceiveTick`
  (params (DeltaSeconds :type "Float (single-precision)"))
  (bind _returnvalue (`self.K2_GetActorLocation`))
  (if (`self.Rotate`)
    ;[1 1 1] Spawn Bleachers
    (`KismetSystemLibrary.Delay` (+ DeltaSeconds (`self.Spawn Delay`)))
    (`|SpawnActorFromClass` "/Game/Blueprints/BP_Bleachers_Rotated.BP_Bleachers_Rotated_C" (`KismetMathLibrary.MakeTransform` _returnvalue (struct :`Yaw` 180.0)) "Undefined" "MultiplyWithRoot" null null)
    (else
      ;[1 1 1] Spawn Bleachers
      (`KismetSystemLibrary.Delay` (+ DeltaSeconds (`self.Spawn Delay`)))
      (`|SpawnActorFromClass` "/Game/Blueprints/BP_Bleachers.BP_Bleachers_C" (`KismetMathLibrary.MakeTransform` _returnvalue) "Undefined" "MultiplyWithRoot" null null))))

(fn `UserConstructionScript`)