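; Player character Blueprint with leaning, physics-driven jumping and a duck state.
; AdjustLean accumulates input into a clamped actor roll, at half rate while jumping or ducking.
; StartJump clears ducking, enables capsule gravity and applies an upward impulse; overlapping a Ground-tagged actor zeroes velocity, disables gravity and ends the jump.
; StartDuck only acts when Ducking is already true, and Tick prints Jumping for debugging.
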(event `self.ReceiveTick`
  (params (DeltaSeconds :type "Float (single-precision)"))
  (`KismetSystemLibrary.PrintString` (`KismetStringLibrary.Conv_BoolToString` (`self.Jumping`))))

(event `self.ReceiveActorBeginOverlap`
  (params (OtherActor :type "Actor Object Reference"))
  (if (`self.ActorHasTag` OtherActor "Ground")
    (`PrimitiveComponent.SetAllPhysicsLinearVelocity` (`self.CapsuleComponent`) (0.0 0.0 0.0) false)
    (`PrimitiveComponent.SetEnableGravity` (`self.CapsuleComponent`) false)
    (set `self.Jumping` false)))

(fn `AdjustLean`
  (params (InputValue :type "Float (double-precision)"))
  (bind (_returnvalue_roll _returnvalue_pitch _returnvalue_yaw) (`KismetMathLibrary.BreakRotator` (`self.K2_GetActorRotation`)))
  (bind (_returnvalue_roll_2 _returnvalue_pitch_2 _returnvalue_yaw_2) (`KismetMathLibrary.BreakRotator` (`self.K2_GetActorRotation`)))
  (if (or (`self.Jumping`) (`self.Ducking`))
    (bind _output_get (set `self.Lean` (`KismetMathLibrary.FClamp` (+ (`self.Lean`) (* 0.5 InputValue)) -50.0 50.0)))
    (`self.K2_SetActorRotation` (`KismetMathLibrary.MakeRotator` _output_get _returnvalue_pitch_2 _returnvalue_yaw_2))
    (else
      (bind _output_get_2 (set `self.Lean` (`KismetMathLibrary.FClamp` (+ (`self.Lean`) (* 1.0 InputValue)) -50.0 50.0)))
      (`self.K2_SetActorRotation` (`KismetMathLibrary.MakeRotator` _output_get_2 _returnvalue_pitch _returnvalue_yaw)))))

(fn `StartDuck`
  (if (`self.Ducking`)
    (`|ExecutionSequence`
      (:`then_0`
        (if (`self.Jumping`)
          (set `self.Jumping` false)))
      (:`then_1`
        (set `self.Ducking` true)))))

(fn `StartJump`
  (if (not (`self.Jumping`))
    (`|ExecutionSequence`
      (:`then_0`
        (if (`self.Ducking`)
          (set `self.Ducking` false)))
      (:`then_1`
        (`PrimitiveComponent.SetEnableGravity` (`self.CapsuleComponent`) true)
        (`PrimitiveComponent.AddImpulse` (`self.CapsuleComponent`) (0.0 0.0 1000.0) "None" true)
        (set `self.Jumping` true)))))

(fn `UserConstructionScript`)