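; Player controller that adds a Chat widget to the viewport and relays movement input to the CBBA player character.
; BeginPlay creates the widget and caches the B_CBBAInstance game instance.
; Enhanced Input lean, jump and duck actions print debug strings, then call the matching functions on the character fetched by player index 0, not the controlled pawn.
; Lean passes its action value on both Triggered and Ongoing.
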(event `self.ReceiveBeginPlay`
  (bind _returnvalue (`|CreateWidget` "/Game/Chat/UI/Chat.Chat_C" (`GameplayStatics.GetPlayerController` 0)))
  (`UserWidget.AddToViewport` _returnvalue 0)
  (bind _asb_cbbainstance (cast `/Game/Player/Blueprints/B_CBBAInstance` (`GameplayStatics.GetGameInstance`)))
  (set `self.GameInstance` _asb_cbbainstance))

(event `EnhancedInput|/Game/Player/Input/Actions/IA_Lean`
  (params (ActionValue :type "Float (double-precision)") (ElapsedSeconds :type "Float (double-precision)") (TriggeredSeconds :type "Float (double-precision)") (InputAction :type "InputAction Object Reference" :default "/Game/Player/Input/Actions/IA_Lean.IA_Lean"))
  (:`Triggered`
    (`KismetSystemLibrary.PrintString` "Hello1" :!label _label)
    (bind _asb_cbbaplayer_character (cast `/Game/Player/Blueprints/B_CBBAPlayerCharacter` (`GameplayStatics.GetPlayerCharacter` 0)))
    (`/Game/Player/Blueprints/B_CBBAPlayerCharacter.AdjustLean` _asb_cbbaplayer_character ActionValue))
  (:`Ongoing`
    (goto _label)))

(event `EnhancedInput|/Game/Player/Input/Actions/IA_Jump`
  (params (ActionValue :type Boolean) (ElapsedSeconds :type "Float (double-precision)") (TriggeredSeconds :type "Float (double-precision)") (InputAction :type "InputAction Object Reference" :default "/Game/Player/Input/Actions/IA_Jump.IA_Jump"))
  (:`Started`
    (`KismetSystemLibrary.PrintString` "Hello2")
    (bind _asb_cbbaplayer_character (cast `/Game/Player/Blueprints/B_CBBAPlayerCharacter` (`GameplayStatics.GetPlayerCharacter` 0)))
    (`/Game/Player/Blueprints/B_CBBAPlayerCharacter.StartJump` _asb_cbbaplayer_character)))

(event `EnhancedInput|/Game/Player/Input/Actions/IA_Duck`
  (params (ActionValue :type Boolean) (ElapsedSeconds :type "Float (double-precision)") (TriggeredSeconds :type "Float (double-precision)") (InputAction :type "InputAction Object Reference" :default "/Game/Player/Input/Actions/IA_Duck.IA_Duck"))
  (:`Started`
    (`KismetSystemLibrary.PrintString` "Hello3")
    (bind _asb_cbbaplayer_character (cast `/Game/Player/Blueprints/B_CBBAPlayerCharacter` (`GameplayStatics.GetPlayerCharacter` 0)))
    (`/Game/Player/Blueprints/B_CBBAPlayerCharacter.StartDuck` _asb_cbbaplayer_character)))

(fn `UserConstructionScript`)